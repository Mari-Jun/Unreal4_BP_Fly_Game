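; Roth_BP is a shop actor, apparently a vendor, that shows and hides the item shop screen for the player.
; On BeginPlay it creates and caches an ItemShopUI widget, passing the player's Hero as Visitor.
; Open Inter displays it with mouse cursor, Game-and-UI input and a click sound.
; Close Inter removes it, restores game-only input, hides the cursor and unpauses, though opening never pauses.
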(event EventBeginPlay
  (bind _ashero (Utilities|Casting|CastToHero (Game|GetPlayerCharacter 0)))
  (bind _returnvalue (UserInterface|CreateWidget "/Game/Prototype/ETC/Shop/ItemShopUI.ItemShopUI_C" 0 _ashero))
  (Variables|Default|SetUI _returnvalue))

(event Collision|EventActorBeginOverlap
  (params (OtherActor :type Actor%20Object%20Reference)))

(event EventTick
  (params (DeltaSeconds :type Float%20%28single-precision%29)))

(fn ConstructionScript)

(fn CloseInter
  (bind _returnvalue (Game|GetPlayerController 0))
  (Widget|RemovefromParent (Variables|Default|GetUI))
  (Input|SetInputModeGameOnly _returnvalue)
  (Game|SetGamePaused false)
  (Variables|/Script/Engine.PlayerController|SetbShowMouseCursor _returnvalue false)
  (return true))

(fn OpenInter
  (bind _returnvalue (Game|GetPlayerController 0))
  (UserInterface|Viewport|AddtoViewport (Variables|Default|GetUI) 0)
  (Input|SetInputModeGameandUI _returnvalue 0 "DoNotLock" true)
  (Variables|/Script/Engine.PlayerController|SetbShowMouseCursor _returnvalue true)
  (Audio|PlaySoundatLocation "/Engine/VREditor/Sounds/VR_click1.VR_click1" (Transformation|GetActorLocation) "0, 0, 0" 1.0 1.0 0.0 0 0 0)
  (return true))