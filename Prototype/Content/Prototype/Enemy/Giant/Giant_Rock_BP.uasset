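; Giant_Rock_BP is a destructible rock projectile, apparently thrown by the Giant enemy.
; Spawn holds it without physics or collision; Throw enables physics and applies an impulse along the given direction with an upward lift.
; On hit it damages a Hero if that is what it struck, then shatters the destructible along its Arrow's forward vector.
; The debris switches its collision object type to Visibility and the actor destroys itself after a short delay.
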(event OnComponentHit(DestructibleComponent)
  (params (HitComponent :type Primitive%20Component%20Object%20Reference) (OtherActor :type Actor%20Object%20Reference) (OtherComp :type Primitive%20Component%20Object%20Reference) (NormalImpulse :type Vector :default "0, 0, 0") (Hit :type Hit%20Result%20Structure%20%28by%20ref%29))
  (bind _arrow (Variables|Default|GetArrow))
  (bind _ashero (Utilities|Casting|CastToHero OtherActor)
    (:then
      (Game|Damage|ApplyDamage _ashero (Variables|Default|GetDamage) 0 self))
    (:CastFailed
      _))
  (Class|DestructibleComponent|ApplyDamage (Variables|Default|GetDestructibleComponent) 1e+03 (Transformation|GetWorldLocation _arrow) (Math|Vector|GetForwardVector _arrow) 1e+03)
  (Collision|SetCollisionObjectType (Variables|Default|GetDestructibleComponent) "ECC_Visibility")
  (Utilities|FlowControl|Delay 3.0)
  (Actor|DestroyActor))

(event EventBeginPlay)

(event Collision|EventActorBeginOverlap
  (params (OtherActor :type Actor%20Object%20Reference)))

(event EventTick
  (params (DeltaSeconds :type Float%20%28single-precision%29)))

(event EventThrow
  (params (Direction :type Vector :default "0, 0, 0"))
  (bind _destructiblecomponent (Variables|Default|GetDestructibleComponent))
  (Collision|SetCollisionEnabled _destructiblecomponent "PhysicsOnly")
  (Physics|SetSimulatePhysics _destructiblecomponent true)
  (Physics|AddImpulse _destructiblecomponent (+ (* Direction 1.5e+04) "0, 0,15000.000000") "None" false))

(fn ConstructionScript)

(fn Spawn
  (bind _destructiblecomponent (Variables|Default|GetDestructibleComponent))
  (Physics|SetSimulatePhysics _destructiblecomponent false)
  (Collision|SetCollisionEnabled _destructiblecomponent "NoCollision")
  (return true))