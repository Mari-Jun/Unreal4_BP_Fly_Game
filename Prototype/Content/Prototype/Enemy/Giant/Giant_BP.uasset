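; Giant enemy Blueprint that configures a parent enemy class with two attack and three skill montages, each with its own damage, plus skill delay ranges.
; OnWeaponBeginOverlap enables overlap events on the left, right or both weapons according to the current attack or skill index.
; SpawnRock attaches a skill-damage rock to a mesh socket, and ThrowRock releases it along the controller's forward vector.
; DeathEnemy plays a death animation before running the parent's death logic.
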(event Custom|Throw%20Rock
  ;[1 1 1] Attack
  (Utilities|IsValid (Variables|Default|GetRock)
    (:Is%20Valid
      (Transformation|DetachFromActor (Variables|Default|GetRock) "KeepWorld" "KeepWorld" "KeepWorld")
      (Class|GiantInter|Throw(Message) (Variables|Default|GetRock) (Transformation|GetActorForwardVector (Pawn|GetController)))
      (Variables|Default|SetRock 0))))

(event Custom|Spawn%20Rock
  ;[1 1 1] Attack
  (bind _returnvalue (Game|SpawnActorfromClass "/Game/Prototype/Enemy/Giant/Giant_Rock_BP.Giant_Rock_BP_C" (Transformation|GetWorldTransform (Variables|Character|GetMesh)) "Undefined" 0 (Utilities|Array|Get(acopy) (Variables|Default|GetDamageSkill) (Variables|Default|GetSkillIndex)) 0))
  (bind _success (Class|GiantInter|Spawn(Message) _returnvalue))
  (if _success
    (bind _output_get (Variables|Default|SetRock _returnvalue))
    (Transformation|AttachComponentToComponent _output_get (Variables|Character|GetMesh) "RockSocket" "SnapToTarget" "SnapToTarget" "KeepWorld" true)))

(event Custom|On%20Weapon%20Begin%20Overlap
  ;[1 1 1] Overlap Weapon
  (switch int (Variables|Default|GetAttackIndex)
    (:Default
      (switch int (Variables|Default|GetSkillIndex)
        (:0
          (Variables|/Script/Engine.PrimitiveComponent|SetbGenerateOverlapEvents (Variables|Default|GetLeftWeapon) true)
          (Variables|/Script/Engine.PrimitiveComponent|SetbGenerateOverlapEvents (Variables|Default|GetRightWeapon) true))
        (:2
          (Variables|/Script/Engine.PrimitiveComponent|SetbGenerateOverlapEvents (Variables|Default|GetRightWeapon) true :!label _label))))
    (:0
      (Variables|/Script/Engine.PrimitiveComponent|SetbGenerateOverlapEvents (Variables|Default|GetLeftWeapon) true))
    (:1
      (goto _label))))

(event EventBeginPlay
  (bind _damage (Variables|Default|GetDamage))
  (bind _damage_2 (Variables|Default|GetDamage))
  (bind _returnvalue (* _damage 2.0))
  (|CallParentFunction)
  ;[1 1 1] Init
  (Variables|Default|SetWeaponCols (Utilities|Array|MakeArray (Variables|Default|GetRightWeapon) (Variables|Default|GetLeftWeapon)))
  (CallFunction|InitWeaponCollision)
  (Variables|Default|SetAttackMontage (Utilities|Array|MakeArray "/Game/Prototype/Enemy/Giant/Giant_Attack_A.Giant_Attack_A" "/Game/Prototype/Enemy/Giant/Giant_Attack_B.Giant_Attack_B"))
  (Variables|Default|SetDamageIndex (Utilities|Array|MakeArray _damage_2 _damage_2))
  (Variables|Default|SetSkillMontage (Utilities|Array|MakeArray "/Game/Prototype/Enemy/Giant/Giant_Skill_A.Giant_Skill_A" "/Game/Prototype/Enemy/Giant/Giant_Skill_B.Giant_Skill_B" "/Game/Prototype/Enemy/Giant/Giant_Skill_C.Giant_Skill_C"))
  (Variables|Default|SetDamageSkill (Utilities|Array|MakeArray _returnvalue _returnvalue (* _damage 1.5)))
  (Variables|Default|SetMinSkillDelay (Utilities|Array|MakeArray 5.0 8.0 3.0))
  (Variables|Default|SetMaxSkillDelay (Utilities|Array|MakeArray 1e+01 12.0 5.0)))

(event Collision|EventActorBeginOverlap
  (params (OtherActor :type Actor%20Object%20Reference))
  (|CallParentFunction OtherActor) ; This node is disabled and will not be called.\nDrag off pins to build functionality.
)

(event EventTick
  (params (DeltaSeconds :type Float%20%28single-precision%29))
  (|CallParentFunction DeltaSeconds) ; This node is disabled and will not be called.\nDrag off pins to build functionality.
)

(fn ConstructionScript
  (|CallParentFunction))

(fn DeathEnemy
  (bind _array (Utilities|Array|MakeArray "/Game/Prototype/Enemy/Giant/ExoGame_Giant_Death_.ExoGame_Giant_Death_"))
  (Components|Animation|PlayAnimation (Variables|Character|GetMesh) (Utilities|Array|Get(acopy) _array (Math|Random|RandomIntegerinRange 0 (- (Utilities|Array|Length _array) 1))) false)
  (|CallParentFunction))