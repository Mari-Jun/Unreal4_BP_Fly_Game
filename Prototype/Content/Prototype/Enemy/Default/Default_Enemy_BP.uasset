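; Base enemy character with health bar, random montage attacks, indexed skills and cooldowns ticked down for polling through check functions.
; Weapon overlaps apply per-attack or per-skill damage, skipping heroes registered in a hit list that clears when the weapon window ends.
; Incoming damage updates the bar, reports to AI perception, grants hero XP and plays hit reactions when idle.
; Death unpossesses, disables collision, awards souls and destroys the actor after a delay.
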(event Custom|Skill%20End
  ;[1 1 1] Attack
  (Variables|Default|SetIsSkill false)
  (Variables|Default|SetCurAttackDelay (Math|Random|RandomFloatinRange (Variables|Default|GetMinAttackDelay) (Variables|Default|GetMaxAttackDelay)))
  (|SetBy-RefVar (Utilities|Array|Get(acopy) (Variables|Default|GetCurSkillDelay) (Variables|Default|GetSkillIndex)) (Math|Random|RandomFloatinRange (Utilities|Array|Get(acopy) (Variables|Default|GetMinSkillDelay) (Variables|Default|GetSkillIndex)) (Utilities|Array|Get(acopy) (Variables|Default|GetMaxSkillDelay) (Variables|Default|GetSkillIndex))))
  (Variables|Default|SetSkillIndex -1))

(event Custom|Init%20Weapon%20Collision
  ;[1 1 1] Damage
  (for _array_element (Variables|Default|GetWeaponCols)
    (Collision|BindEventtoOnComponentBeginOverlap _array_element (delegate Custom|Add%20Damage))))

(event Custom|Add%20Damage
  (params (OverlappedComponent :type Primitive%20Component%20Object%20Reference) (OtherActor :type Actor%20Object%20Reference) (OtherComp :type Primitive%20Component%20Object%20Reference) (OtherBodyIndex :type Integer) (bFromSweep :type Boolean) (SweepResult :type Hit%20Result%20Structure%20%28by%20ref%29))
  ;[1 1 1] Damage
  (for _array_element (Variables|Default|GetOverlapCharacter)
    (Variables|Default|SetIsBeforeDamage (or (== _array_element OtherActor) (Variables|Default|GetIsBeforeDamage))))
  (if (Variables|Default|GetIsBeforeDamage)
    (Variables|Default|SetIsBeforeDamage false)
    (elif (Variables|Default|GetIsSkill)
      (CallFunction|ApplyDamage OtherActor (Variables|Default|GetDamageSkill) (Variables|Default|GetSkillIndex))
      (elif (Variables|Default|GetIsAttack)
        (CallFunction|ApplyDamage OtherActor (Variables|Default|GetDamageIndex) (Variables|Default|GetAttackIndex))))))

(event Custom|On%20Weapon%20End%20Overlap
  ;[1 1 1] Overlap Weapon
  (for _array_element (Variables|Default|GetWeaponCols)
    (Variables|/Script/Engine.PrimitiveComponent|SetbGenerateOverlapEvents _array_element false)
    (Utilities|Array|Clear (Variables|Default|GetOverlapCharacter))))

(event Custom|Attack%20End
  ;[1 1 1] Attack
  (Variables|Default|SetIsAttack false)
  (Variables|Default|SetCurAttackDelay (Math|Random|RandomFloatinRange (Variables|Default|GetMinAttackDelay) (Variables|Default|GetMaxAttackDelay)))
  (Variables|Default|SetAttackIndex -1))

(event Custom|Death_Delay
  ;[1 1 1] Death
  (Utilities|FlowControl|Delay 5.0)
  (Actor|DestroyActor))

(event Custom|End%20Hit
  ;[1 1 1] Damage
  (Variables|Default|SetIsAttack false)
  (Variables|Default|SetAttackIndex -1)
  (Variables|Default|SetIsSkill false)
  (Variables|Default|SetSkillIndex -1)
  (Variables|Default|SetCurAttackDelay 0.0))

(event Custom|Add%20Damaged%20Hero
  (params (Hero :type Hero%20Object%20Reference))
  ;[1 1 1] Damaged Hero
  (Utilities|Array|Add (Variables|Default|GetOverlapCharacter) Hero))

(event EventBeginPlay
  (bind _enemyhealthwidget (Variables|Default|GetEnemyHealthWidget))
  (Development|SetHiddeninGame _enemyhealthwidget true false)
  (bind _asenemy_ui (Utilities|Casting|CastToEnemyUI (UserInterface|GetUserWidgetObject _enemyhealthwidget)))
  (Default|UpdateHP _asenemy_ui (/ (Variables|Info|GetHP) (Variables|Info|GetMaxHP))))

(event Collision|EventActorBeginOverlap
  (params (OtherActor :type Actor%20Object%20Reference)))

(event EventTick
  (params (DeltaSeconds :type Float%20%28single-precision%29))
  (bind _curskilldelay (Variables|Default|GetCurSkillDelay))
  (Variables|Default|SetCurAttackDelay (Math|Float|Max(Float) (- (Variables|Default|GetCurAttackDelay) DeltaSeconds) 0.0))
  (for (_array_element _array_index) _curskilldelay
    (|SetBy-RefVar (Utilities|Array|Get(acopy) _curskilldelay _array_index) (Math|Float|Max(Float) (- _array_element DeltaSeconds) 0.0))))

(event EventStartAttack
  ;[1 1 1] Attack
  (Variables|Default|SetIsAttack true)
  (Variables|Default|SetAttackIndex (Math|Random|RandomIntegerinRange 0 (- (Utilities|Array|Length (Variables|Default|GetAttackMontage)) 1)))
  (Animation|PlayAnimMontage (Utilities|Array|Get(acopy) (Variables|Default|GetAttackMontage) (Variables|Default|GetAttackIndex)) 1.0 "None"))

(event Game|Damage|EventAnyDamage
  (params (Damage :type Float%20%28single-precision%29) (DamageType :type Damage%20Type%20Object%20Reference) (InstigatedBy :type Controller%20Object%20Reference) (DamageCauser :type Actor%20Object%20Reference))
  (bind _self self)
  (bind _hitmontage (Variables|Default|GetHitMontage))
  (bind _returnvalue (Utilities|Array|Length _hitmontage))
  ;[1 1 1] Damage
  (CallFunction|UpdateHP Damage)
  (bind _ashero (Utilities|Casting|CastToHero DamageCauser))
  (Default|AddDamagedEnemy _ashero _self)
  (Class|AISenseDamage|ReportDamageEvent _self DamageCauser Damage (Transformation|GetActorLocation))
  (bind _ashero_2 (Utilities|Casting|CastToHero DamageCauser))
  (Default|ComputeXP _ashero_2 (/ Damage 5.0))
  (if (and (Math|Boolean|NORBoolean (Variables|Default|GetIsAttack) (Variables|Default|GetIsSkill)) (> _returnvalue 0))
    (Animation|PlayAnimMontage (Utilities|Array|Get(acopy) (Variables|Default|GetHitMontage) (Math|Random|RandomIntegerinRange 0 (- _returnvalue 1))) 1.0 "None")))

(fn ConstructionScript)

(fn UpdateHP
  (params (Value :type Float%20%28single-precision%29))
  (bind _output_get (Variables|Info|SetHP (- (Variables|Info|GetHP) Value)))
  (bind _asenemy_ui (Utilities|Casting|CastToEnemyUI (UserInterface|GetUserWidgetObject (Variables|Default|GetEnemyHealthWidget))))
  (Default|UpdateHP _asenemy_ui (/ _output_get (Variables|Info|GetMaxHP)))
  (Development|SetHiddeninGame (Variables|Default|GetEnemyHealthWidget) false false)
  (if (<= (Variables|Info|GetHP) 0.0)
    (CallFunction|DeathEnemy)))

(fn ApplyDamage
  (params (DamagedActor :type Actor%20Object%20Reference) (Array :type Array%20of%20Floats%20%28single-precision%29) (Index :type Integer))
  (Game|Damage|ApplyDamage DamagedActor (Utilities|Array|Get(acopy) Array Index) (AI|GetAIController 0) self))

(fn DeathEnemy
  (Utilities|FlowControl|DoOnce false
    (:Completed
      (Pawn|UnPossess (Pawn|GetController))
      (Development|SetHiddeninGame (Variables|Default|GetEnemyHealthWidget) true false)
      (Collision|SetActorEnableCollision false)
      (bind _ashero (Utilities|Casting|CastToHero (Game|GetPlayerCharacter 0)))
      (Default|ComputeSoul _ashero (Variables|Info|GetSoul))
      (CallFunction|DeathDelay))))

(fn CheckAttackEnable
  (return (== (Variables|Default|GetCurAttackDelay) 0.0)))

(fn CheckSKillEnable
  (params (Index :type Integer))
  (return (== (Utilities|Array|Get(acopy) (Variables|Default|GetCurSkillDelay) Index) 0.0)))

(fn EndAttack
  (return (not (Variables|Default|GetIsAttack))))

(fn EndSkill
  (return (not (Variables|Default|GetIsSkill))))

(fn StartSkill
  (params (Index :type Integer))
  (Variables|Default|SetIsSkill true)
  (Variables|Default|SetSkillIndex Index)
  (Animation|PlayAnimMontage (Utilities|Array|Get(acopy) (Variables|Default|GetSkillMontage) (Variables|Default|GetSkillIndex)) 1.0 "None")
  (return))