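; Grunt enemy bomb projectile that explodes on impact and damages the Hero.
; Shoot turns on physics for the mesh and launches it with a fixed-strength impulse along the given direction.
; A mesh hit spawns the explosion effect and sound, then enables the sphere's overlap events for a brief window before the actor destroys itself.
; Any Hero that begins overlapping the sphere takes the bomb's damage.
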(event OnComponentHit(StaticMesh)
  (params (HitComponent :type Primitive%20Component%20Object%20Reference) (OtherActor :type Actor%20Object%20Reference) (OtherComp :type Primitive%20Component%20Object%20Reference) (NormalImpulse :type Vector :default "0, 0, 0") (Hit :type Hit%20Result%20Structure%20%28by%20ref%29))
  (bind _returnvalue (Transformation|GetActorLocation))
  (Effects|SpawnEmitteratLocation "/Game/InfinityBladeEffects/Effects/FX_Monsters/FX_Monster_Gruntling/Bomber/P_FireBombExplosion.P_FireBombExplosion" _returnvalue "0, 0, 0" "2.000000,2.000000,2.000000")
  (Audio|PlaySoundatLocation "/Game/StarterContent/Audio/Explosion02.Explosion02" _returnvalue "0, 0, 0" 1.0 1.0 0.0 0 0 0)
  (Variables|Default|SetBomb true)
  (Variables|/Script/Engine.PrimitiveComponent|SetbGenerateOverlapEvents (Variables|Default|GetSphere) true)
  (Utilities|FlowControl|Delay 0.2)
  (Actor|DestroyActor))

(event OnComponentBeginOverlap(Sphere)
  (params (OverlappedComponent :type Primitive%20Component%20Object%20Reference) (OtherActor :type Actor%20Object%20Reference) (OtherComp :type Primitive%20Component%20Object%20Reference) (OtherBodyIndex :type Integer) (bFromSweep :type Boolean) (SweepResult :type Hit%20Result%20Structure%20%28by%20ref%29))
  (bind _ashero (Utilities|Casting|CastToHero OtherActor))
  (Game|Damage|ApplyDamage _ashero (Variables|Default|GetDamage) 0 self))

(event EventBeginPlay)

(event Collision|EventActorBeginOverlap
  (params (OtherActor :type Actor%20Object%20Reference)))

(event EventTick
  (params (DeltaSeconds :type Float%20%28single-precision%29)))

(event EventShoot
  (params (Direction :type Vector :default "0, 0, 0"))
  (bind _staticmesh (Variables|Default|GetStaticMesh))
  (Collision|SetCollisionEnabled _staticmesh "PhysicsOnly")
  (Physics|SetSimulatePhysics _staticmesh true)
  (Physics|AddImpulse _staticmesh (* Direction 5e+03) "None" false))

(fn ConstructionScript)