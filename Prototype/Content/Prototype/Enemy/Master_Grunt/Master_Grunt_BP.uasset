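; Master Grunt enemy Blueprint that configures a parent enemy class with melee attacks, a bomb skill and its own death animation.
; BeginPlay fills the inherited montage, damage and delay arrays and registers both weapon collisions.
; OnWeaponBeginOverlap enables overlaps on the right, left or both weapons according to the attack index.
; Bomb spawns a projectile at BombArrow with the boosted skill damage, launches it forward and adds a muzzle flash.
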(event Custom|Bomb
  ;[1 1 1] Attack
  (bind _returnvalue (Game|SpawnActorfromClass "/Game/Prototype/Enemy/Master_Grunt/Master_Grunt_Bomb_BP.Master_Grunt_Bomb_BP_C" (Math|Transform|MakeTransform (Transformation|GetWorldLocation (Variables|Default|GetBombArrow)) "0, 0, 0" "0.300000,0.300000,0.300000") "Undefined" 0 (Utilities|Array|Get(acopy) (Variables|Default|GetDamageSkill)) 0))
  (Class|MGFireInter|Shoot(Message) _returnvalue (Math|Vector|GetForwardVector (Variables|Default|GetBombArrow)))
  (Effects|SpawnEmitterAttached "/Game/InfinityBladeEffects/Effects/FX_Monsters/FX_Monster_Gruntling/Master/P_BackPack_MuzzleFlash.P_BackPack_MuzzleFlash" (Variables|Default|GetBombArrow) "None"))

(event Custom|On%20Weapon%20Begin%20Overlap
  ;[1 1 1] Overlap Weapon
  (switch int (Variables|Default|GetAttackIndex)
    (:0
      (Variables|/Script/Engine.PrimitiveComponent|SetbGenerateOverlapEvents (Variables|Default|GetRightWeapon) true)
      (Variables|/Script/Engine.PrimitiveComponent|SetbGenerateOverlapEvents (Variables|Default|GetLeftWeapon) true))
    (:1
      (Variables|/Script/Engine.PrimitiveComponent|SetbGenerateOverlapEvents (Variables|Default|GetRightWeapon) true))
    (:2
      (Variables|/Script/Engine.PrimitiveComponent|SetbGenerateOverlapEvents (Variables|Default|GetLeftWeapon) true))))

(event EventBeginPlay
  (bind _damage (Variables|Default|GetDamage))
  (|CallParentFunction)
  ;[1 1 1] Init
  (Variables|Default|SetWeaponCols (Utilities|Array|MakeArray (Variables|Default|GetRightWeapon) (Variables|Default|GetLeftWeapon)))
  (CallFunction|InitWeaponCollision)
  (Variables|Default|SetAttackMontage (Utilities|Array|MakeArray "/Game/Prototype/Enemy/Master_Grunt/Master_Grunt_AttackA.Master_Grunt_AttackA" "/Game/Prototype/Enemy/Master_Grunt/Master_Grunt_AttackB.Master_Grunt_AttackB" "/Game/Prototype/Enemy/Master_Grunt/Master_Grunt_AttackC.Master_Grunt_AttackC"))
  (Variables|Default|SetDamageIndex (Utilities|Array|MakeArray _damage _damage _damage))
  (Variables|Default|SetMinAttackDelay 1.0)
  (Variables|Default|SetMaxAttackDelay 1.5)
  (Variables|Default|SetSkillMontage (Utilities|Array|MakeArray "/Game/Prototype/Enemy/Master_Grunt/Master_Grunt_SkillA.Master_Grunt_SkillA"))
  (Variables|Default|SetDamageSkill (Utilities|Array|MakeArray (* (Variables|Default|GetDamage) 2.5)))
  (Variables|Default|SetMinSkillDelay (Utilities|Array|MakeArray 4.0))
  (Variables|Default|SetMaxSkillDelay (Utilities|Array|MakeArray 6.0))
  (Variables|Default|SetHitMontage (Utilities|Array|MakeArray "/Game/Prototype/Enemy/Master_Grunt/Master_Grunt_Hit.Master_Grunt_Hit")))

(event Collision|EventActorBeginOverlap
  (params (OtherActor :type Actor%20Object%20Reference))
  (|CallParentFunction OtherActor) ; This node is disabled and will not be called.\nDrag off pins to build functionality.
)

(event EventTick
  (params (DeltaSeconds :type Float%20%28single-precision%29))
  (|CallParentFunction DeltaSeconds) ; This node is disabled and will not be called.\nDrag off pins to build functionality.
)

(fn ConstructionScript
  (|CallParentFunction))

(fn DeathEnemy
  (bind _array (Utilities|Array|MakeArray "/Game/InfinityBladeAdversaries/Enemy/Enemy_Master_Grunt/Enemy_Master_Grunt_Animation/ExoGame_MasterGrunt_Death.ExoGame_MasterGrunt_Death"))
  (Components|Animation|PlayAnimation (Variables|Character|GetMesh) (Utilities|Array|Get(acopy) _array (Math|Random|RandomIntegerinRange 0 (- (Utilities|Array|Length _array) 1))) false)
  (|CallParentFunction))