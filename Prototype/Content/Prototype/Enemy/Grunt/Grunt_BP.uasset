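; Grunt enemy Blueprint for a bomb-carrying gruntling that turns into a timed explosive when set on fire, extending a parent enemy class.
; Burning raises its speed, shows the particle effect and starts a Tick countdown that fires Bomb once if it is still alive.
; Bomb plays explosion effects, hides the bomb bone, enables the explosion collider registered as its weapon collision, and passes its own HP to UpdateHP.
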(event Custom|On%20Start%20Burn
  ;[1 1 1] Attack
  (Variables|/Script/Engine.CharacterMovementComponent|SetMaxWalkSpeed (Variables|Character|GetCharacterMovement) 6e+02)
  (Variables|Default|SetIs%20Bomb true)
  (Development|SetHiddeninGame (Variables|Default|GetParticleSystem) false false))

(event EventBeginPlay
  (|CallParentFunction)
  ;[1 1 1] Init
  (Variables|Default|SetWeaponCols (Utilities|Array|MakeArray (Variables|Default|GetExplosion%20Col)))
  (CallFunction|InitWeaponCollision)
  (Variables|Default|SetDamageIndex (Utilities|Array|MakeArray (Variables|Default|GetDamage)))
  (Variables|Default|SetAttackIndex 0))

(event Collision|EventActorBeginOverlap
  (params (OtherActor :type Actor%20Object%20Reference))
  (|CallParentFunction OtherActor) ; This node is disabled and will not be called.\nDrag off pins to build functionality.
)

(event EventTick
  (params (DeltaSeconds :type Float%20%28single-precision%29))
  (|CallParentFunction DeltaSeconds)
  (if (Variables|Default|GetIs%20Bomb)
    (bind _output_get (Variables|Default|SetBomb%20Time (- (Variables|Default|GetBomb%20Time) DeltaSeconds)))
    (if (and (< _output_get 0.0) (> (Variables|Default|GetHP) 0.0))
      (Utilities|FlowControl|DoOnce false
        (:Completed
          (CallFunction|Bomb))))))

(event EventStartAttack
  ;[1 1 1] Attack
  (Utilities|FlowControl|DoOnce false
    (:Completed
      (Variables|Default|SetIsAttack true)
      (Variables|/Script/Engine.CharacterMovementComponent|SetMaxWalkSpeed (Variables|Character|GetCharacterMovement) 0.0))))

(fn ConstructionScript
  (|CallParentFunction))

(fn DeathEnemy
  (Components|Animation|PlayAnimation (Variables|Character|GetMesh) "/Game/InfinityBladeAdversaries/Enemy/Enemy_Gruntling_Avalanche/Enemy_Gruntling_Avalanche_Animation/ExoGame_Gruntling_Death_Small_05.ExoGame_Gruntling_Death_Small_05" false)
  (|CallParentFunction))

(fn Bomb
  (bind _particlesystem (Variables|Default|GetParticleSystem))
  (bind _returnvalue (Transformation|GetWorldLocation _particlesystem))
  (Development|SetHiddeninGame _particlesystem true false)
  (Effects|SpawnEmitteratLocation "/Game/InfinityBladeEffects/Effects/FX_Monsters/FX_Monster_Gruntling/Bomber/P_FireBombExplosion.P_FireBombExplosion" _returnvalue "0, 0, 0" "2.500000,2.500000,2.500000")
  (Audio|PlaySoundatLocation "/Game/StarterContent/Audio/Explosion01.Explosion01" _returnvalue "0, 0, 0" 1.0 1.0 0.0 0 0 0)
  (Components|SkinnedMesh|HideBonebyName (Variables|Character|GetMesh) "b_MF_Bomb" "PBO_None")
  (Variables|/Script/Engine.PrimitiveComponent|SetbGenerateOverlapEvents (Variables|Default|GetExplosion%20Col) true)
  (CallFunction|UpdateHP (Variables|Default|GetHP)))