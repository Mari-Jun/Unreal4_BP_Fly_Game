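; Zombie enemy that chases the player's ShootBP pawn once it comes within range.
; Each Tick measures the distance to the player, sets the IsMove and IsAttack range flags, and computes a look-at rotation.
; When IsMove is set, it moves along its forward vector and snaps to that rotation, with no navigation pathfinding.
; IsAttack is only set here; the graph contains no attack logic.
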(event EventBeginPlay)

(event Collision|EventActorBeginOverlap
  (params (OtherActor :type Actor%20Object%20Reference)))

(event EventTick
  (params (DeltaSeconds :type Float%20%28single-precision%29))
  (bind _returnvalue (Transformation|GetActorLocation))
  (Utilities|FlowControl|Sequence
    (:then_0
      (bind _asshoot_bp (Utilities|Casting|CastToShootBP (Game|Player|GetPlayerPawn 0)))
      (bind _output_get (Variables|Default|SetDistance (Math|Vector|Distance(Vector) _returnvalue (Transformation|GetActorLocation _asshoot_bp))))
      (Variables|Default|SetIsMove (< _output_get 2.5e+03))
      (Variables|Default|SetIsAttack (< _output_get 1e+03))
      (Variables|Default|SetRotation (Math|Rotator|FindLookatRotation _returnvalue (Transformation|GetActorLocation _asshoot_bp))))
    (:then_1
      (if (Variables|Default|GetIsMove)
        (Pawn|Input|AddMovementInput (Transformation|GetActorForwardVector) 1.0 false)
        (Transformation|SetActorRotation (Variables|Default|GetRotation))))))

(event EventEndPlay
  (params (EndPlayReason :type EEndPlayReason%20Enum :default "Destroyed")))

(fn ConstructionScript)