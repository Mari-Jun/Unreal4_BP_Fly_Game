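; Ball_BP is a throwable physics ball actor in the FPS Zombie folder.
; Spawn puts it in an inert state by turning off mesh physics and all collision on the mesh and sphere.
; Throw re-enables mesh physics and query-only sphere collision, launches the mesh with a directional impulse plus upward lift, then destroys the actor after a short delay.
; No overlap or damage logic is implemented here.
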(event EventBeginPlay)

(event Collision|EventActorBeginOverlap
  (params (OtherActor :type Actor%20Object%20Reference)))

(event EventTick
  (params (DeltaSeconds :type Float%20%28single-precision%29)))

(event EventThrow
  (params (Direction :type Vector :default "0, 0, 0"))
  (bind _staticmesh (Variables|Default|GetStaticMesh))
  (Collision|SetCollisionEnabled (Variables|Default|GetSphere) "QueryOnly")
  (Collision|SetCollisionEnabled _staticmesh "PhysicsOnly")
  (Physics|SetSimulatePhysics _staticmesh true)
  (Physics|AddImpulse _staticmesh (+ (* Direction 1.5e+03) "0, 0,300.000000") "None" false)
  (Utilities|FlowControl|Delay 5.0)
  (Actor|DestroyActor))

(fn ConstructionScript)

(fn Spawn
  (bind _staticmesh (Variables|Default|GetStaticMesh))
  (Physics|SetSimulatePhysics _staticmesh false)
  (Collision|SetCollisionEnabled _staticmesh "NoCollision")
  (Collision|SetCollisionEnabled (Variables|Default|GetSphere) "NoCollision")
  (return true))