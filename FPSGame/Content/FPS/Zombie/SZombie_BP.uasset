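; Ranged zombie enemy for a shooter that plays a throw montage when the player is near and faces them while attacking.
; SpawnBall and Throw, not called within this Blueprint, attach a ball to a hand-held socket and launch it forward.
; Point damage lowers HP, with headshots killing instantly; death plays an animation, reports to ShootBP and destroys the actor.
; A health widget tracks the zombie through world-to-screen projection.
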(event EventBeginPlay
  (bind _returnvalue (UserInterface|CreateWidget "/Game/FPS/Zombie/ZombieUI.ZombieUI_C" 0 self))
  (bind _output_get (Variables|Default|SetUI _returnvalue))
  (UserInterface|Viewport|AddtoViewport _output_get 0)
  (Variables|Default|SetHP (Variables|Default|GetMaxHP))
  (Default|CallUpdateHP (Utilities|GetHPPercent))
  (Class|UserWidget|SetPositioninViewport (Variables|Default|GetUI) (.ScreenLocation (Class|PlayerController|ProjectWorldLocationtoScreen (Game|GetPlayerController 0) (+ (Transformation|GetActorLocation) "0, 0,100.000000") false)) true))

(event Collision|EventActorBeginOverlap
  (params (OtherActor :type Actor%20Object%20Reference)))

(event EventTick
  (params (DeltaSeconds :type Float%20%28single-precision%29))
  (bind _returnvalue (Transformation|GetActorLocation))
  (bind _returnvalue_2 (Transformation|GetActorLocation))
  (bind _returnvalue_3 (Game|GetPlayerController 0))
  (bind _returnvalue_4 (+ _returnvalue "0, 0,100.000000"))
  (bind (_screenlocation _returnvalue_5) (Class|PlayerController|ProjectWorldLocationtoScreen _returnvalue_3 _returnvalue_4 false))
  (Utilities|FlowControl|Sequence
    (:then_0
      (bind _asshoot_bp (Utilities|Casting|CastToShootBP (Game|Player|GetPlayerPawn 0)))
      (bind _output_get (Variables|Default|SetDistance (Math|Vector|Distance(Vector) _returnvalue_2 (Transformation|GetActorLocation _asshoot_bp))))
      (if (and (< _output_get 1e+03) (not (Utilities|IsHPZero)))
        (if (Variables|Default|GetIsAttack)
          (Transformation|SetActorRotation (Math|Rotator|FindLookatRotation _returnvalue_2 (Transformation|GetActorLocation _asshoot_bp)))
          (else
            (Variables|Default|SetIsAttack true)
            (Animation|Montage|PlayMontage (Variables|Character|GetMesh) "/Game/FPS/Zombie/ThrowMontage.ThrowMontage"
              (:OnCompleted
                (Variables|Default|SetIsAttack false)))))))
    (:then_1
      (if (and (not (Audio|Components|Audio|IsPlaying (Variables|Character|GetMesh))) (Utilities|IsHPZero))
        (Utilities|FlowControl|DoOnce false
          (:Completed
            (Utilities|FlowControl|Delay 1.0)
            (Actor|DestroyActor)))))
    (:then_2
      (if _returnvalue_5
        (Class|UserWidget|SetPositioninViewport (Variables|Default|GetUI) _screenlocation true)))))

(event Game|Damage|EventPointDamage
  (params (Damage :type Float%20%28single-precision%29) (DamageType :type Damage%20Type%20Object%20Reference) (HitLocation :type Vector :default "0, 0, 0") (HitNormal :type Vector :default "0, 0, 0") (HitComponent :type Primitive%20Component%20Object%20Reference) (BoneName :type Name :default "None") (ShotFromDirection :type Vector :default "0, 0, 0") (InstigatedBy :type Controller%20Object%20Reference) (DamageCauser :type Actor%20Object%20Reference) (HitInfo :type Hit%20Result%20Structure%20%28by%20ref%29))
  (if (Utilities|Name|Equal(Name) BoneName "Head")
    (Variables|Default|SetHP 0.0)
    (Default|CallUpdateHP (Utilities|GetHPPercent))
    (Components|Animation|PlayAnimation (Variables|Character|GetMesh) "/Game/Zombie/Animation/Zombie_Dying.Zombie_Dying" false :!label _label)
    (Collision|SetActorEnableCollision false)
    (bind _asshoot_bp (Utilities|Casting|CastToShootBP (Game|Player|GetPlayerPawn 0)))
    (Utilities|FlowControl|Delay 1.2)
    (Default|CheckZombieCount _asshoot_bp 1)
    (else
      (bind _output_get (Variables|Default|SetHP (- (Variables|Default|GetHP) Damage)))
      (Default|CallUpdateHP (Utilities|GetHPPercent))
      (if (<= _output_get 0.0)
        (goto _label)))))

(event EventEndPlay
  (params (EndPlayReason :type EEndPlayReason%20Enum :default "Destroyed"))
  (bind _ball (Variables|Default|GetBall))
  (Widget|RemovefromParent (Variables|Default|GetUI))
  (Utilities|IsValid _ball
    (:Is%20Valid
      (Actor|DestroyActor _ball))))

(fn ConstructionScript)

(fn Throw
  (Utilities|IsValid (Variables|Default|GetBall)
    (:Is%20Valid
      (Transformation|DetachFromActor (Variables|Default|GetBall) "KeepWorld" "KeepWorld" "KeepWorld")
      (Class|BallInter|Throw(Message) (Variables|Default|GetBall) (Transformation|GetActorForwardVector))
      (Variables|Default|SetBall 0))))

(fn SpawnBall
  (bind _returnvalue (Game|SpawnActorfromClass "/Game/FPS/Zombie/Ball_BP.Ball_BP_C" (Transformation|GetWorldTransform (Variables|Character|GetMesh)) "Undefined" 0 0))
  (bind _success (Class|BallInter|Spawn(Message) _returnvalue))
  (if _success
    (bind _output_get (Variables|Default|SetBall _returnvalue))
    (Transformation|AttachComponentToComponent _output_get (Variables|Character|GetMesh) "BallSocket" "SnapToTarget" "SnapToTarget" "KeepWorld" true)))