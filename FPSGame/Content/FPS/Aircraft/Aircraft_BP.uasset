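; Aircraft that flies forward on its own and carries the player's ShootBP pawn until Space destroys it.
; Tick feeds a delta-scaled forward vector into FloatingPawnMovement.
; SetPlayerLocation snaps the player pawn just above the aircraft with matching rotation at BeginPlay and every tick, without attaching it.
; BeginPlay enables input so Space can destroy the aircraft, ending that position lock.
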(event EventBeginPlay
  (Input|EnableInput (Game|GetPlayerController 0))
  (CallFunction|SetPlayerLocation))

(event Collision|EventActorBeginOverlap
  (params (OtherActor :type Actor%20Object%20Reference)))

(event EventTick
  (params (DeltaSeconds :type Float%20%28single-precision%29))
  (Class|PawnMovementComponent|AddInputVector (Variables|Default|GetFloatingPawnMovement) (* (Transformation|GetActorForwardVector) (* DeltaSeconds 1e+04)) false)
  (CallFunction|SetPlayerLocation))

(event Input|KeyboardEvents|SpaceBar
  (params (Key :type Key%20Structure :default "None"))
  (:Pressed
    (Actor|DestroyActor)))

(fn ConstructionScript)

(fn SetPlayerLocation
  (bind _returnvalue (Game|Player|GetPlayerPawn 0))
  (Utilities|Casting|CastToShootBP _returnvalue)
  (Transformation|SetActorLocationAndRotation _returnvalue (+ (Transformation|GetActorLocation) "0, 0,100.000000") (Transformation|GetActorRotation)))