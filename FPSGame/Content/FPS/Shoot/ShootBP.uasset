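; Player character for a zombie shooter with health, ammo and grenade HUD, sprint, and gun pickups.
; Fire and throw inputs play montages and manage weapon attachment or visibility, while separate functions, not called here, handle hitscan shots and grenade spawn and release.
; Tick feeds movement values and opens the paused restart screen when no zombies remain or the first fall nears Landscape without G clearing it; lethal ball hits also open it.
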(event OnComponentBeginOverlap(CapsuleComponent)
  (params (OverlappedComponent :type Primitive%20Component%20Object%20Reference) (OtherActor :type Actor%20Object%20Reference) (OtherComp :type Primitive%20Component%20Object%20Reference) (OtherBodyIndex :type Integer) (bFromSweep :type Boolean) (SweepResult :type Hit%20Result%20Structure%20%28by%20ref%29))
  (bind _success (Class|WeaponInter|Grab(Message) OtherActor))
  (if _success
    (Utilities|IsValid (Variables|Default|GetWeapon_Gun)
      (:Is%20Valid
        (Actor|DestroyActor OtherActor))
      (:Is%20Not%20Valid
        (bind _output_get (Variables|Default|SetWeapon_Gun OtherActor))
        (Transformation|AttachComponentToComponent _output_get (Variables|Character|GetMesh) "GunSocket" "SnapToTarget" "SnapToTarget" "KeepWorld" true)))
    (bind _output_get_2 (Variables|Default|SetBulletCount (+ (Variables|Default|GetBulletCount) 30)))
    (Default|CallChangeBulletCount _output_get_2)))

(event OnComponentHit(CapsuleComponent)
  (params (HitComponent :type Primitive%20Component%20Object%20Reference) (OtherActor :type Actor%20Object%20Reference) (OtherComp :type Primitive%20Component%20Object%20Reference) (NormalImpulse :type Vector :default "0, 0, 0") (Hit :type Hit%20Result%20Structure%20%28by%20ref%29))
  (bind _asball_bp (Utilities|Casting|CastToBall_BP OtherActor))
  (Actor|DestroyActor _asball_bp)
  (bind _output_get (Variables|Default|SetHP (- (Variables|Default|GetHP) 1e+02)))
  (Default|CallHPUpdate (/ _output_get (Variables|Default|GetMaxHP)))
  (if (<= (Variables|Default|GetHP) 0.0)
    (CallFunction|RestartGame)))

(event EventBeginPlay
  (bind _maxhp (Variables|Default|GetMaxHP))
  (Utilities|FlowControl|Sequence
    (:then_0
      (bind _outactors (Actor|GetAllActorsOfClass "/Game/FPS/Zombie/SZombie_BP.SZombie_BP_C"))
      (Variables|Default|SetZombieCount (Utilities|Array|Length _outactors)))
    (:then_1
      (bind _returnvalue (UserInterface|CreateWidget "/Game/FPS/Shoot/ShootUI.ShootUI_C" 0 self))
      (bind _output_get (Variables|Default|SetUI _returnvalue))
      (UserInterface|Viewport|AddtoViewport _output_get 0)
      (bind _output_get_2 (Variables|Default|SetHP _maxhp))
      (Default|CallHPUpdate (/ _output_get_2 _maxhp))
      (Default|CallChangeBulletCount (Variables|Default|GetBulletCount))
      (Default|CallChangeGrenadeCount (Variables|Default|GetGrenadeCount)))))

(event Collision|EventActorBeginOverlap
  (params (OtherActor :type Actor%20Object%20Reference)))

(event EventTick
  (params (DeltaSeconds :type Float%20%28single-precision%29))
  (bind _charactermovement (Variables|Character|GetCharacterMovement))
  (Utilities|FlowControl|Sequence
    (:then_0
      (Variables|Default|SetDirection (Class|KismetMathLibrary|DegAtan2 (Input|AxisValues|GetMOVE_FORWARD) (Input|AxisValues|GetMOVE_RIGHT)))
      (Variables|Default|SetSpeed (Math|Vector|VectorLength (* (Transformation|GetVelocity) "1.000000,1.000000, 0"))))
    (:then_1
      (Variables|/Script/Engine.CharacterMovementComponent|SetMaxWalkSpeed _charactermovement (Math|Float|Clamp(Float) (+ (Variables|/Script/Engine.CharacterMovementComponent|GetMaxWalkSpeed _charactermovement) (* (Utilities|Time|GetWorldDeltaSeconds) (Variables|Default|GetSpeedChangeValue))) 3e+02 6e+02))
      (if (== (Variables|Default|GetZombieCount) 0)
        (CallFunction|RestartGame)))
    (:then_2
      (bind _hit_actor (CallFunction|Crash 1e+02))
      (Utilities|Casting|CastToLandscape _hit_actor)
      (if (Variables|Default|GetFirstFall)
        (CallFunction|RestartGame)))))

(event EventEndPlay
  (params (EndPlayReason :type EEndPlayReason%20Enum :default "Destroyed"))
  (Widget|RemovefromParent (Variables|Default|GetUI)))

(event Input|ActionEvents|InputActionSPRINT
  (params (Key :type Key%20Structure :default "None"))
  (:Pressed
    (Variables|Default|SetSpeedChangeValue 3e+02))
  (:Released
    (Variables|Default|SetSpeedChangeValue -3e+02)))

(event Input|ActionEvents|InputActionFIRE
  (params (Key :type Key%20Structure :default "None"))
  (bind _weapon_gun (Variables|Default|GetWeapon_Gun))
  (:Pressed
    (Utilities|IsValid _weapon_gun
      (:Is%20Valid
        (if (and (> (Variables|Default|GetBulletCount) 0) (not (Variables|Default|GetIsThrow)))
          (Variables|Default|SetIsFire true)
          (Animation|PlayAnimMontage "/Game/FPS/Shoot/ShootingMontage.ShootingMontage" 1.0 "None")
          (Transformation|AttachComponentToComponent (Variables|Default|GetWeapon_Gun) (Variables|Character|GetMesh) "GunShootSocket" "SnapToTarget" "SnapToTarget" "KeepWorld" true)))))
  (:Released
    (Utilities|IsValid _weapon_gun
      (:Is%20Valid
        (if (Variables|Default|GetIsFire)
          (Variables|Default|SetIsFire false)
          (Variables|Default|SetIsThrow false)
          (Animation|StopAnimMontage "/Game/FPS/Shoot/ShootingMontage.ShootingMontage")
          (Transformation|AttachComponentToComponent (Variables|Default|GetWeapon_Gun) (Variables|Character|GetMesh) "GunSocket" "SnapToTarget" "SnapToTarget" "KeepWorld" true))))))

(event Input|ActionEvents|InputActionJUMP
  (params (Key :type Key%20Structure :default "None"))
  (:Pressed
    (Character|Jump))
  (:Released
    (Character|StopJumping)))

(event Input|ActionEvents|InputActionTHROW
  (params (Key :type Key%20Structure :default "None"))
  (bind _weapon_gun (Variables|Default|GetWeapon_Gun))
  (bind _weapon_gun_2 (Variables|Default|GetWeapon_Gun))
  (:Pressed
    (if (not (Variables|Default|GetIsThrow))
      (if (> (Variables|Default|GetGrenadeCount) 0)
        (Variables|Default|SetIsThrow true)
        (Utilities|IsValid _weapon_gun_2
          (:Is%20Valid
            (Rendering|SetActorHiddenInGame _weapon_gun_2 true))
          (:Is%20Not%20Valid
            _))
        (Animation|Montage|PlayMontage (Variables|Character|GetMesh) "/Game/FPS/Shoot/ThrowMontage.ThrowMontage"
          (:OnCompleted
            (Variables|Default|SetIsThrow false)
            (Utilities|IsValid _weapon_gun
              (:Is%20Valid
                (Rendering|SetActorHiddenInGame _weapon_gun false)))))))))

(event Input|KeyboardEvents|G
  (params (Key :type Key%20Structure :default "None"))
  (:Pressed
    (bind _hit_actor (CallFunction|Crash 2e+03))
    (Utilities|Casting|CastToLandscape _hit_actor)
    (Variables|Default|SetFirstFall false)))

(fn ConstructionScript)

(fn Shoot
  (bind _returnvalue (Pawn|GetControlRotation :!class /Script/Engine.Pawn))
  (bind _springarm (Variables|Default|GetSpringArm))
  (bind _returnvalue_2 (Transformation|GetWorldLocation _springarm))
  (bind _returnvalue_3 (Math|Vector|GetForwardVector _returnvalue))
  (bind _result (Math|Integer|DecrementInt (Variables|Default|GetBulletCount))
    (:%20%20
      (Default|CallChangeBulletCount _result)
      (bind (_outhit _returnvalue_4) (Collision|LineTraceByChannel _returnvalue_2 (+ _returnvalue_2 (* _returnvalue_3 5e+03)) "TraceTypeQuery1" false 0 "None"))
      (if _returnvalue_4
        (Effects|SpawnEmitteratLocation 0 (.Location (Collision|BreakHitResult _outhit)))
        (Utilities|Casting|CastToBoX_BP (.HitActor (Collision|BreakHitResult _outhit))
          (:CastFailed
            (Game|Damage|ApplyPointDamage (.HitActor (Collision|BreakHitResult _outhit)) 1e+02 _returnvalue_3 _outhit (Pawn|GetController))))))))

(fn RestartGame
  (bind _returnvalue (Game|GetPlayerController 0))
  (bind _returnvalue_2 (UserInterface|CreateWidget "/Game/FPS/RestatrUI.RestatrUI_C"))
  (UserInterface|Viewport|AddtoViewport _returnvalue_2 0)
  (Input|SetInputModeGameandUI _returnvalue 0 "DoNotLock" true)
  (Variables|/Script/Engine.PlayerController|SetbShowMouseCursor _returnvalue true)
  (Game|SetGamePaused true))

(fn CheckZombieCount
  (params (ChangeValue :type Integer))
  (Variables|Default|SetZombieCount (- (Variables|Default|GetZombieCount) ChangeValue)))

(fn IncreaseGrenadeCount
  (bind _result (Math|Integer|IncrementInt (Variables|Default|GetGrenadeCount))
    (:%20%20
      (bind _output_get (Variables|Default|SetGrenadeCount _result))
      (Default|CallChangeGrenadeCount _output_get))))

(fn Throw
  (bind _result (Math|Integer|DecrementInt (Variables|Default|GetGrenadeCount))
    (:%20%20
      (Variables|Default|SetGrenadeCount _result)
      (Utilities|IsValid (Variables|Default|GetWeapon_Grenade)
        (:Is%20Valid
          (Transformation|DetachFromActor (Variables|Default|GetWeapon_Grenade) "KeepWorld" "KeepWorld" "KeepWorld")
          (Class|GrenadeInter|Throw(Message) (Variables|Default|GetWeapon_Grenade) (Transformation|GetActorForwardVector (Pawn|GetController)))
          (Variables|Default|SetWeapon_Grenade 0)
          (Default|CallChangeGrenadeCount (Variables|Default|GetGrenadeCount)))))))

(fn SpawnGrenade
  (bind _returnvalue (Game|SpawnActorfromClass "/Game/FPS/Shoot/Grenade.Grenade_C" (Transformation|GetWorldTransform (Variables|Character|GetMesh)) "Undefined" 0 0))
  (bind _success (Class|GrenadeInter|Spawn(Message) _returnvalue))
  (if _success
    (bind _output_get (Variables|Default|SetWeapon_Grenade _returnvalue))
    (Transformation|AttachComponentToComponent _output_get (Variables|Character|GetMesh) "GrenadeSocket" "SnapToTarget" "SnapToTarget" "KeepWorld" true)))

(fn Crash
  (params (Length :type Float%20%28single-precision%29))
  (bind _returnvalue (Transformation|GetActorLocation))
  (if (Variables|Default|GetFirstFall)
    (bind (_outhit _returnvalue_2) (Collision|LineTraceByChannel _returnvalue (+ _returnvalue (* "0, 0,-1.000000" Length)) "TraceTypeQuery1" false 0 "None"))
    (if _returnvalue_2
      (return (.HitActor (Collision|BreakHitResult _outhit))))))